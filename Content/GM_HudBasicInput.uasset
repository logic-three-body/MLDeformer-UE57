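; Game mode for an ML Deformer demo that creates stat, button-help and message HUDs and adds the keyboard/gamepad input mapping.
; After a short timer for stat groups, Tick feeds the stat widget GPU morph time, ML inference time and flesh, shirt and pants deformer memory.
; Events toggle HUD visibility and wireframe-plus-bones show flags via console commands.
; Helper functions forward messages, play state and orbit-camera state to the widgets.
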(event Custom|StatGroupsReady
  ;[1 1 1] Create HUD and Set Control
  (Variables|Default|SetStatGroupInitiailized true))

(event Custom|ToggleHUD
  ;[1 1 1] HUD Visibility
  (CallFunction|ToggleWidgetVisibility (Variables|Default|GetStatWidget)))

(event Custom|ToggleButtonHelpHUD
  ;[1 1 1] HUD Visibility
  (CallFunction|ToggleWidgetVisibility (Variables|Default|GetButtonHelpWidget)))

(event Custom|ToggleShowWireframe
  (CallFunction|ToggleWireframe))

(event EventBeginPlay
  ;[1 1 1] Create HUD and Set Control
  (CallFunction|CreateStatHUD)
  (CallFunction|CreateButtonHelpHUD)
  (CallFunction|CreateMessageHUD)
  (Input|AddMappingContext (PlayerController|LocalPlayerSubsystems|GetEnhancedInputLocalPlayerSubsystem (Game|GetPlayerController 0)) "/Game/Input/KeyboardGamepadMapping.KeyboardGamepadMapping" 0 "(bIgnoreAllPressedKeysUntilRelease=True,bForceImmediately=False)")
  (Development|ExecuteConsoleCommand "DisableAllScreenMessages" 0)
  (Utilities|Time|SetTimerbyEvent (delegate Custom|StatGroupsReady) 0.1))

(event EventTick
  (params (DeltaSeconds :type Float%20%28single-precision%29))
  (bind _returnvalue (* 1024.0 1024.0))
  (bind _statwidget (Variables|Default|GetStatWidget))
  ;[1 1 1] Monitor Performance Stats
  (if (Variables|Default|GetStatGroupInitiailized)
    (Variables|/Game/UI/WBP_StatHUD.WBP_StatHUD_C|SetMorphMS _statwidget (Class|MLDeformerSampleGameModeBase|GetGPUMorphTargetTimeMS))
    (Variables|/Game/UI/WBP_StatHUD.WBP_StatHUD_C|SetMLDeformerMS _statwidget (Class|MLDeformerSampleGameModeBase|GetMLInferenceTime))
    (Variables|/Game/UI/WBP_StatHUD.WBP_StatHUD_C|SetFleshMemoryMB _statwidget (/ (Math|Conversions|ToFloat(Integer) (Class|MLDeformerSampleGameModeBase|GetMLGPUMemoryinBytes "FleshDeformer")) _returnvalue))
    (Variables|/Game/UI/WBP_StatHUD.WBP_StatHUD_C|SetShirtMemoryMB _statwidget (/ (Math|Conversions|ToFloat(Integer) (Class|MLDeformerSampleGameModeBase|GetMLGPUMemoryinBytes "ShirtDeformer")) _returnvalue))
    (Variables|/Game/UI/WBP_StatHUD.WBP_StatHUD_C|SetPantsMemoryMB _statwidget (/ (Math|Conversions|ToFloat(Integer) (Class|MLDeformerSampleGameModeBase|GetMLGPUMemoryinBytes "PantsDeformer")) _returnvalue))))

(fn ConstructionScript)

(fn CreateStatHUD
  (bind _returnvalue (UserInterface|CreateWidget "/Game/UI/WBP_StatHUD.WBP_StatHUD_C"))
  (bind _output_get (Variables|Default|SetStatWidget _returnvalue))
  (if (Class|MLDeformerSampleGameModeBase|IsShippingBuild)
    (Variables|Default|SetHudIndex 3))
  (UserInterface|Viewport|AddtoViewport _output_get 0)
  (Variables|/Game/UI/WBP_StatHUD.WBP_StatHUD_C|SetHeaderColour _output_get (Variables|Default|GetHudHeaderColor))
  (Variables|/Game/UI/WBP_StatHUD.WBP_StatHUD_C|SetTextColour _output_get (Variables|Default|GetHudTextColor))
  (Default|SetHudIndex _output_get (Variables|Default|GetHudIndex))
  (Default|SetHudOpacity _output_get (Variables|Default|GetHudOpacity))
  (Widget|SetVisibility _output_get "Visible")
  (return 0))

(fn CreateButtonHelpHUD
  (bind _returnvalue (UserInterface|CreateWidget "/Game/UI/WBP_ButtonHelpHUD.WBP_ButtonHelpHUD_C"))
  (bind _output_get (Variables|Default|SetButtonHelpWidget _returnvalue))
  (UserInterface|Viewport|AddtoViewport _output_get 0)
  (Widget|SetVisibility _output_get "Hidden")
  (return 0))

(fn ToggleWidgetVisibility
  (params (Widget :type Widget%20Object%20Reference%20%28by%20ref%29))
  (if (Widget|IsVisible Widget)
    (Widget|SetVisibility Widget "Hidden")
    (else
      (Widget|SetVisibility Widget "Visible"))))

(fn ToggleWireframe
  (bind _output_get (Variables|Default|SetShowingWireframe (not (Variables|Default|GetShowingWireframe))))
  (if _output_get
    (Development|ExecuteConsoleCommand "ShowFlag.WireFrame 1" 0)
    (Development|ExecuteConsoleCommand "ShowFlag.Bones 1" 0)
    (else
      (Development|ExecuteConsoleCommand "ShowFlag.WireFrame 0" 0)
      (Development|ExecuteConsoleCommand "ShowFlag.Bones 0" 0))))

(fn CreateMessageHUD
  (bind _returnvalue (UserInterface|CreateWidget "/Game/UI/WBP_MessageHUD.WBP_MessageHUD_C"))
  (bind _output_get (Variables|Default|SetMessageHUD _returnvalue))
  (UserInterface|Viewport|AddtoViewport _output_get 0)
  (return 0))

(fn ShowMessageonHUD
  (params (Message :type Text))
  (Default|SetMessage (Variables|Default|GetMessageHUD) Message))

(fn SetPlaying
  (params (IsPlaying :type Boolean))
  (Default|SetPlaying (Variables|Default|GetButtonHelpWidget) IsPlaying))

(fn SetOrbitCamera
  (params (Orbit :type Boolean))
  (Default|SetOrbit (Variables|Default|GetButtonHelpWidget) Orbit))