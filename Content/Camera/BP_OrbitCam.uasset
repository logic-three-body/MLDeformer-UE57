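; Orbit camera actor that yaws around a raised pivot and dollies along its local X axis within clamped limits.
; Each Tick scales the orbit and dolly weights by frame delta for FPS-independent speed, then accumulates them into rotation and distance.
; A curve derives camera pitch from dolly distance, so tilt follows zoom.
; The file only consumes these weights and contains no input handling.
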(event EventBeginPlay)

(event Collision|EventActorBeginOverlap
  (params (OtherActor :type Actor%20Object%20Reference)))

(event EventTick
  (params (DeltaSeconds :type Float%20%28single-precision%29))
  (bind _returnvalue (Math|Float|MapRangeUnclamped DeltaSeconds 0.00825 0.066 0.5 4.0))
  (Utilities|FlowControl|Sequence
    (:then_0
      ;[1 1 1] Scale input weights based on tick delta (makes orbitCam speed independent of FPS)
      (Variables|Default|SetDelta_weight_multiply _returnvalue)
      (Variables|Default|SetOrbit_weight (* (Variables|Default|GetOrbit_weight) _returnvalue))
      (Variables|Default|SetDolly_weight (* (Variables|Default|GetDolly_weight) _returnvalue)))
    (:then_1
      ;[1 1 1] Accumulate orbit control weights
      (Variables|Default|SetOrbit_rotate_value (+ (Variables|Default|GetOrbit_rotate_value) (Variables|Default|GetOrbit_weight)))
      (bind _output_get (Variables|Default|SetOrbit_dolly_value (Math|Float|Clamp(Float) (+ (Variables|Default|GetOrbit_dolly_value) (Variables|Default|GetDolly_weight)) -7e+02 -1.6e+02)))
      (Variables|Default|SetOrbit%20_tilt_value (Math|Curves|GetFloatValue (Variables|Default|GetDollyTiltCurve) _output_get)))
    (:then_2
      ;[1 1 1] Apply transforms
      (Transformation|SetRelativeLocationAndRotation (Variables|Default|GetCameraRoot) "0.000000,0.000000,90.000000" (Math|Rotator|MakeRotator 0.0 0.0 (Variables|Default|GetOrbit_rotate_value)) false false)
      (Transformation|SetRelativeLocationAndRotation (Variables|Default|GetOrbitCamera) (Math|Vector|MakeVector (Variables|Default|GetOrbit_dolly_value) 0.0 4e+01) (Math|Rotator|MakeRotator 0.0 (Variables|Default|GetOrbit%20_tilt_value) 0.0) false false))))

(fn ConstructionScript
  (Variables|Default|SetOrbit_rotate_value 9e+01)
  (Variables|Default|SetOrbit_dolly_value -3.6e+02))